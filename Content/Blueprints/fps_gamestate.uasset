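; Game state for an FPS zombie wave mode, tracking the current round and zombie count.
; BeginPlay caches the game mode and player character.
; IncreaseRound advances the round, computes a linearly scaled, capped zombie count and pushes both to the HUD's round display.
; CheckIfRoundIsOver asks the game mode to start a new round once that count reaches zero.
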(event `self.ReceiveBeginPlay`
  (bind _asfps_gamemode (cast `/Game/Blueprints/Fps_gamemode` (`GameplayStatics.GetGameMode`)))
  (set `self.GamemodeRef` _asfps_gamemode)
  (bind _asfps_char (cast `/Game/Blueprints/Fps_char` (`GameplayStatics.GetPlayerPawn` 0)))
  (set `self.PlayerRef` _asfps_char))

(fn `CheckIfRoundIsOver`
  (if (<= (`self.NumberOfZombiesToSpawn`) 0)
    (`/Game/Blueprints/Fps_gamemode.StartNewRound` (`self.GamemodeRef`))))

(fn `IncreaseRound`
  (`/Engine/EditorBlueprintResources/StandardMacros.IncrementInt` (`self.CurrentRound`)
    (:`  `
      (bind _output_get (set `self.NumberOfZombiesToSpawn` (`KismetMathLibrary.Clamp` (`KismetMathLibrary.Round` (+ (* (`self.CurrentRound`) 1.5) 9.0)) 0 150)))
      (`/Game/Blueprints/UMG/UI_RoundNumber.UpdateData` (`/Game/Blueprints/UMG/MainHUD.UI_RoundNumber` (`/Game/Blueprints/Fps_char.MainHUDRef` (`self.PlayerRef`))) (`self.CurrentRound`) _output_get))))

(fn `UserConstructionScript`)