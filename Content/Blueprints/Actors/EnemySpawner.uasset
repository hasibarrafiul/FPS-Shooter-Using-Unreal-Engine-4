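; Enemy spawner actor that creates AI zombies at its own transform and adds them to the game state's zombie count.
; SpawnZombie spawns AI_Character_Child with its behavior tree, ignoring collision, increments NumberOfZombies on the game state cached at BeginPlay, and zeroes the zombie's StartGoalLocation.
; The construction script positions the StartGoalLocation component from GoalVector and GoalRotator, but its world location is never passed to spawned zombies.
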(event `self.ReceiveBeginPlay`
  (bind _asfps_gamestate (cast `/Game/Blueprints/fps_gamestate` (`GameplayStatics.GetGameState`)))
  (set `self.GameStateRef` _asfps_gamestate))

(event `SpawnZombie`
  (bind _returnvalue (`AIBlueprintHelperLibrary.SpawnAIFromClass` "/Game/AI/AI_Character_Child.AI_Character_Child_C" "/Game/AI/AI_BehaviourTree.AI_BehaviourTree" (.location (`self.GetTransform`)) (.rotation (`self.GetTransform`)) true null))
  (`/Engine/EditorBlueprintResources/StandardMacros.IncrementInt` (`/Game/Blueprints/fps_gamestate.NumberOfZombies` (`self.GameStateRef`))
    (:`  `
      (bind _asai_character_child (cast `/Game/AI/AI_Character_Child` _returnvalue))
      (set `/Game/AI/AI_Character.StartGoalLocation` (0.0 0.0 0.0) _asai_character_child))))

(fn `UserConstructionScript`
  (`SceneComponent.K2_SetRelativeLocationAndRotation` (`self.StartGoalLocation`) (`self.GoalVector`) (`self.GoalRotator`) false false))