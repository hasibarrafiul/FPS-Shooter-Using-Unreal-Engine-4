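; Game mode for a round-based zombie FPS that starts rounds and drives enemy spawning.
; On BeginPlay it caches the Fps_gamestate and all EnemySpawner actors, then calls StartNewRound, which waits briefly before increasing the round on the game state.
; A looping timer then spawns zombies at random spawners until the game state's zombie count reaches the round's target, when the timer is cleared.
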(event `self.ReceiveBeginPlay`
  (bind _asfps_gamestate (cast `/Game/Blueprints/fps_gamestate` (`GameplayStatics.GetGameState`)))
  (set `self.GamestateRef` _asfps_gamestate)
  (bind _outactors (`GameplayStatics.GetAllActorsOfClass` "/Game/Blueprints/Actors/EnemySpawner.EnemySpawner_C"))
  (set `self.EnemySpawners` _outactors)
  (`self.StartNewRound`))

(event `StartNewRound`
  (`KismetSystemLibrary.Delay` 5.0)
  (`/Game/Blueprints/fps_gamestate.IncreaseRound` (`self.GamestateRef`))
  (bind _returnvalue (`KismetSystemLibrary.K2_SetTimerDelegate` (delegate `SpawnZombies`) 2.5 true)))

(event `SpawnZombies`
  (bind _gamestateref (`self.GamestateRef`))
  (bind _enemyspawners (`self.EnemySpawners`))
  (if (< (`/Game/Blueprints/fps_gamestate.NumberOfZombies` _gamestateref) (`/Game/Blueprints/fps_gamestate.NumberOfZombiesToSpawn` _gamestateref))
    (`/Game/Blueprints/Actors/EnemySpawner.SpawnZombie` (`|GetArrayItem` _enemyspawners (`KismetMathLibrary.RandomIntegerInRange` 0 (- (`KismetArrayLibrary.Array_Length` _enemyspawners) 1))))
    (else
      (`KismetSystemLibrary.K2_ClearAndInvalidateTimerHandle` (stale `StartNewRound` _returnvalue)))))

(fn `UserConstructionScript`)